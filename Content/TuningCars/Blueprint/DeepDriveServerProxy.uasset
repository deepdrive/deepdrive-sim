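; DeepDrive server proxy Blueprint that relays external client and agent requests to the player-pawn car.
; Requesting control switches off the Car's game driving and sets IsControlled, which gates control input and resets; releasing control reverses both.
; Client registration and capture-camera creation forward to the AliceGT pawn, with camera registration returning the result or 0 if the cast fails.
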(event EventBeginPlay)

(event Collision|EventActorBeginOverlap
  (params (OtherActor :type Actor%20Object%20Reference)))

(event EventRegisterClient
  (params (ClientId :type Integer) (IsMaster :type Boolean))
  (bind _asalice_gt (Utilities|Casting|CastToAliceGT (Game|Player|GetPlayerPawn 0)))
  (Default|RegisterClient _asalice_gt ClientId IsMaster))

(event EventTick
  (params (DeltaSeconds :type Float%20%28single-precision%29)))

(event EventReleaseAgentControl
  (Variables|Default|SetIsControlled false)
  (bind _ascar (Utilities|Casting|CastToCar (Game|Player|GetPlayerPawn 0)))
  (Class|Car|SetIsGameDriving _ascar true)
  (Variables|Default|SetReleaseCounter (+ (Variables|Default|GetReleaseCounter) 1)))

(event EventSetAgentControlValues
  (params (steering :type Float%20%28single-precision%29) (throttle :type Float%20%28single-precision%29) (brake :type Float%20%28single-precision%29) (handbrake :type Boolean))
  (Utilities|FlowControl|Sequence
    (:then_0
      (if handbrake
        (Variables|Default|Set_handbrake 1.0)
        (else
          (Variables|Default|Set_handbrake 0.0))))
    (:then_1
      (if (Variables|Default|GetIsControlled)
        (bind _ascar (Utilities|Casting|CastToCar (Game|Player|GetPlayerPawn 0)))
        (Class|Car|SetControls _ascar steering throttle brake (Variables|Default|Get_handbrake))))))

(event EventUnregisterClient
  (params (ClientId :type Integer) (IsMaster :type Boolean))
  (bind _asalice_gt (Utilities|Casting|CastToAliceGT (Game|Player|GetPlayerPawn 0)))
  (Default|UnregisterClient _asalice_gt))

(event EventResetAgent
  (if (Variables|Default|GetIsControlled)
    (bind _ascar (Utilities|Casting|CastToCar (Game|Player|GetPlayerPawn 0)))
    (Class|Car|SetShouldReset _ascar true)))

(fn ConstructionScript)

(fn RequestAgentControl
  (Variables|Default|SetRequestCounter (+ (Variables|Default|GetRequestCounter) 1))
  (bind _ascar (Utilities|Casting|CastToCar (Game|Player|GetPlayerPawn 0))
    (:then
      (Class|Car|SetIsGameDriving _ascar false)
      (bind _output_get (Variables|Default|SetIsControlled true))
      (return _output_get))
    (:CastFailed
      (return false))))

(fn RegisterCamera
  (params (FieldOfView :type Float%20%28single-precision%29) (CaptureWidth :type Integer) (CaptureHeight :type Integer) (RelativePosition :type Vector) (RelativeRotation :type Vector))
  (bind _asalice_gt (Utilities|Casting|CastToAliceGT (Game|Player|GetPlayerPawn 0))
    (:then
      (bind _cameraid (Default|AddCaptureCamera _asalice_gt FieldOfView CaptureWidth CaptureHeight RelativePosition RelativeRotation))
      (return _cameraid))
    (:CastFailed
      (return 0))))