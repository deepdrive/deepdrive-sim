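; DummyAliceGT is a dummy AliceGT car that randomizes its paint color and tuning parts in the construction script.
; RandomChoice picks meshes for one shared wheel style, both bumpers, wing and hood; the molding pick is not wired into its SetStaticMesh call.
; SetColorToAllCarPaintMaterials applies the random color to body and parts, excluding wheels, through dynamic instances replacing each Carpaint_Inst slot.
; The event graph holds no active logic.
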(event EventBeginPlay)

(event Collision|EventActorBeginOverlap
  (params (OtherActor :type Actor%20Object%20Reference)))

(event EventTick
  (params (DeltaSeconds :type Float%20%28single-precision%29)))

(fn ConstructionScript
  (bind _bumber_rear (Variables|Default|Getbumber_rear))
  (bind _wing (Variables|Default|Getwing))
  (bind _bumper_front (Variables|Default|Getbumper_front))
  (bind _molding (Variables|Default|Getmolding))
  (bind _hood (Variables|Default|Gethood))
  (Utilities|FlowControl|Sequence
    (:then_0
      (Variables|Default|SetCarColor (Math|Color|MakeColor (Math|Random|RandomFloatinRange 0.0 1.0) (Math|Random|RandomFloatinRange 0.0 1.0) (Math|Random|RandomFloatinRange 0.0 1.0)))
      (CallFunction|SetColortoAllCarPaintMaterials (Variables|Default|GetAliceGT)))
    (:then_1
      (bind _tuningitem (CallFunction|RandomChoice (Variables|Default|Getwheels)))
      (Utilities|FlowControl|Sequence
        (:then_0
          (Components|StaticMesh|SetStaticMesh (Variables|Default|Getwheel1) (.mesh _tuningitem)))
        (:then_1
          (Components|StaticMesh|SetStaticMesh (Variables|Default|Getwheel2) (.mesh _tuningitem)))
        (:then_2
          (Components|StaticMesh|SetStaticMesh (Variables|Default|Getwheel3) (.mesh _tuningitem)))
        (:then_3
          (Components|StaticMesh|SetStaticMesh (Variables|Default|Getwheel4) (.mesh _tuningitem)))))
    (:then_2
      (bind _tuningitem_2 (CallFunction|RandomChoice (Variables|Default|Getfront_bumpers)))
      (Components|StaticMesh|SetStaticMesh _bumper_front (.mesh _tuningitem_2))
      (CallFunction|SetColortoAllCarPaintMaterials _bumper_front))
    (:then_3
      (CallFunction|RandomChoice (Variables|Default|Getmoldings))
      (Components|StaticMesh|SetStaticMesh _molding 0)
      (CallFunction|SetColortoAllCarPaintMaterials _molding))
    (:then_4
      (bind _tuningitem_3 (CallFunction|RandomChoice (Variables|Default|Getwings)))
      (Components|StaticMesh|SetStaticMesh _wing (.mesh _tuningitem_3))
      (CallFunction|SetColortoAllCarPaintMaterials _wing))
    (:then_5
      (bind _tuningitem_4 (CallFunction|RandomChoice (Variables|Default|Gethoods)))
      (Components|StaticMesh|SetStaticMesh _hood (.mesh _tuningitem_4))
      (CallFunction|SetColortoAllCarPaintMaterials _hood))
    (:then_6
      (bind _tuningitem_5 (CallFunction|RandomChoice (Variables|Default|Getrear_bumpers)))
      (Components|StaticMesh|SetStaticMesh _bumber_rear (.mesh _tuningitem_5))
      (CallFunction|SetColortoAllCarPaintMaterials _bumber_rear))))

(fn RandomChoice
  (params (Array :type Array%20of%20Tuning%20Item%20Structures))
  (bind _returnvalue (Utilities|Array|Length Array))
  (if (> _returnvalue 0)
    (return (Utilities|Array|Get(acopy) Array (Math|Random|RandomIntegerinRange 0 (- _returnvalue 1))))
    (else
      (return ""))))

(fn SetColortoAllCarPaintMaterials
  (params (Component :type Mesh%20Component%20Object%20Reference))
  (for (_array_element _array_index) (Rendering|Material|GetMaterials Component)
    (if (== _array_element "/Game/TuningCars/Materials/carpaint_Inst.carpaint_Inst")
      (bind _returnvalue (Rendering|Material|CreateDynamicMaterialInstance Component _array_index "/Game/TuningCars/Materials/carpaint_Inst.carpaint_Inst" :!class /Script/Engine.PrimitiveComponent))
      (Rendering|Material|SetVectorParameterValue _returnvalue (Variables|Default|GetColorParameter) (Variables|Default|GetCarColor) :!class /Script/Engine.MaterialInstanceDynamic))))