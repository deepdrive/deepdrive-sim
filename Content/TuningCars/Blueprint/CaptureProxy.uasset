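; CaptureProxy supplies DeepDrive capture data from the player's car.
; BeginPlay casts player pawn 0 to Car and caches it.
; BeginCapture packs that car's motion, dimensions, control inputs, driving and reset state, and route, lane and lap progress into a DeepDriveDataOut struct.
; The Brake field is filled from the physics handbrake getter, while Handbrake takes the car's last applied handbrake value.
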(event EventBeginPlay
  (bind _ascar (Utilities|Casting|CastToCar (Game|Player|GetPlayerPawn 0)))
  (Variables|Default|SetCar _ascar))

(fn ConstructionScript)

(fn BeginCapture
  (bind _car (Variables|Default|GetCar))
  (bind _returnvalue (Transformation|GetActorTransform _car))
  (return (Utilities|Struct|MakeDeepDriveDataOut (.location _returnvalue) (.rotation _returnvalue) (Transformation|GetVelocity _car) (Variables|/Script/DeepDrive.Car|GetAcceleration _car) (Class|Car|GetAngularVelocity _car) (Variables|/Script/DeepDrive.Car|GetAngularAcceleration _car) (Variables|/Script/DeepDrive.Car|GetDimension _car) (Vehicle|GetForwardSpeed (Variables|/Script/Engine.WheeledVehicle|GetVehicleMovement _car)) (Class|Car|GetIsGameDriving _car) (Class|Car|GetIsResetting _car) (Class|Car|GetPhysicsSteering _car) (Class|Car|GetPhysicsThrottle _car) (Class|Car|GetPhysicsHandbrake _car) (Variables|/Script/DeepDrive.Car|GetLastAppliedHandbrake _car) (Variables|/Script/DeepDrive.Car|GetDistanceAlongRoute _car) (Variables|/Script/DeepDrive.Car|GetDistanceToCenterOfLane _car) (Variables|/Script/DeepDrive.Car|GetLapNumber _car))))