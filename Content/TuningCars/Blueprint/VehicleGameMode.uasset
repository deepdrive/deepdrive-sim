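; VehicleGameMode is the game mode that sets up the driving session when play begins.
; It creates a hidden pause menu and a top-layer loading screen, then blocking-loads and flushes the Canyons streaming level.
; Once loaded, it moves the player's AliceGT car to the initial transform and flags it for reset, then fades out the loading screen and fades in the vehicle HUD.
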(event EventBeginPlay
  (Utilities|FlowControl|Sequence
    (:then_0
      (bind _returnvalue (UserInterface|CreateWidget "/Game/TuningCars/Blueprint/HUD/PauseGUI.PauseGUI_C"))
      (UserInterface|Viewport|AddtoViewport _returnvalue 0)
      (Widget|SetVisibility _returnvalue "Hidden"))
    (:then_1
      (bind _returnvalue_2 (UserInterface|CreateWidget "/Game/TuningCars/Blueprint/HUD/LoadingScreenWidget.LoadingScreenWidget_C"))
      (bind _output_get (Variables|Default|SetLoadingScreen _returnvalue_2))
      (UserInterface|Viewport|AddtoViewport _output_get 1000))
    (:then_2
      (Game|LoadStreamLevel(byName) "Canyons" true true)
      (Class|GameplayStatics|FlushLevelStreaming)
      (bind _asalice_gt (Utilities|Casting|CastToAliceGT (Game|Player|GetPlayerPawn 0)))
      (Default|SetCarTransform _asalice_gt (Variables|Default|GetInitialCarTransform))
      (Class|Car|SetShouldReset _asalice_gt true)
      (Default|FadeOut (Variables|Default|GetLoadingScreen) 2.0)
      (bind _asvehicle_hud (Utilities|Casting|CastToVehicleHUD (HUD|GetHUD (Game|GetPlayerController 0))))
      (Default|Fadein (Variables|/Game/TuningCars/Blueprint/HUD/VehicleHUD.VehicleHUD_C|GetVehicleHUD _asvehicle_hud)))))

(fn ConstructionScript)