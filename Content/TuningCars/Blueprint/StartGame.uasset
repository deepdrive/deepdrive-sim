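; StartGame is the startup Blueprint that builds the tuning game's UI on BeginPlay.
; It adds the main menu, plus hidden pause and tuning-menu widgets, to the viewport, storing the tuning menu on TuningCar_GameInst.
; It then calls LoadCanyonsEvent on the main menu to load the hangar.
; A car-creation fragment that clears the GameInstance's Car and calls Possess is unconnected and never runs.
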(event EventBeginPlay
  (bind _returnvalue (Game|GetPlayerController 0))
  (Utilities|FlowControl|Sequence
    (:then_1
      ;[1 1 1] Create Widgets
      (bind _returnvalue_2 (UserInterface|CreateWidget "/Game/TuningCars/Blueprint/HUD/main_menu.main_menu_C" _returnvalue))
      (UserInterface|Viewport|AddtoViewport _returnvalue_2 0)
      (Variables|Default|Setmain%20menu _returnvalue_2)
      (bind _returnvalue_3 (UserInterface|CreateWidget "/Game/TuningCars/Blueprint/HUD/PauseGUI.PauseGUI_C"))
      (UserInterface|Viewport|AddtoViewport _returnvalue_3 0)
      (Widget|SetVisibility _returnvalue_3 "Hidden"))
    (:then_2
      (bind _returnvalue_4 (UserInterface|CreateWidget "/Game/TuningCars/Blueprint/HUD/menu_tuning.menu_tuning_C" _returnvalue))
      (bind _astuning_car_game_inst (Utilities|Casting|CastToTuningCar_GameInst (Game|GetGameInstance)))
      (bind _output_get (Variables|/Game/TuningCars/Blueprint/TuningCar_GameInst.TuningCar_GameInst_C|Setmenu_tuning _astuning_car_game_inst _returnvalue_4))
      (UserInterface|Viewport|AddtoViewport _output_get 0)
      (Widget|SetVisibility _output_get "Hidden"))
    (:then_3
      ;[1 1 1] load hangar
      (Default|LoadCanyonsEvent (Variables|Default|Getmain%20menu)))))

(fn ConstructionScript)