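; DeepDrive control proxy that relays incoming control data to the player's Car pawn.
; It caches the pawn on BeginPlay, then forwards steering, throttle, brake and handbrake on every OnNewControlData event.
; The game-driving and reset flags are cached locally and pushed to the car only when they change.
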(event EventOnNewControlData
  (params (controlData :type Deep%20Drive%20Control%20Data%20Structure%20%28by%20ref%29))
  (bind (_steering _throttle _brake _handbrake _isgamedriving _shouldreset) (Utilities|Struct|BreakDeepDriveControlData controlData))
  (Utilities|FlowControl|Sequence
    (:then_0
      (if (Math|Boolean|NotEqual(Boolean) (Variables|Default|GetIsGameDriving) _isgamedriving)
        (Variables|Default|SetIsGameDriving _isgamedriving)
        (Class|Car|SetIsGameDriving (Variables|Default|GetCar) _isgamedriving)))
    (:then_1
      (Class|Car|SetControls (Variables|Default|GetCar) _steering _throttle _brake _handbrake))
    (:then_2
      (if (Math|Boolean|NotEqual(Boolean) (Variables|Default|GetShouldReset) _shouldreset)
        (Variables|Default|SetShouldReset _shouldreset)
        (Class|Car|SetShouldReset (Variables|Default|GetCar) _shouldreset)))))

(event EventBeginPlay
  (bind _ascar (Utilities|Casting|CastToCar (Game|Player|GetPlayerPawn 0)))
  (bind _output_get (Variables|Default|SetCar _ascar)))

(fn ConstructionScript)