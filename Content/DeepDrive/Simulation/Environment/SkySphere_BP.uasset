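; Sky sphere Blueprint for the DeepDrive simulation environment that renders an atmospheric scattering sky.
; The construction script creates a dynamic material on the sphere mesh and feeds it a lookup texture generated by SunLightSimulator.
; UpdateSunDirection passes the SunLight actor's forward vector to that material as the sun direction.
; Unconnected leftovers of an older color-driven sky with panning clouds and stars never run.
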(fn ConstructionScript
  (bind _returnvalue (Rendering|Material|CreateDynamicMaterialInstance (Variables|BP_Skydome|GetSkySphereMesh) 0 "/Game/DeepDrive/Simulation/Environment/M_AtmosphericScatteringSky_Master.M_AtmosphericScatteringSky_Master" :!class /Script/Engine.PrimitiveComponent))
  (Variables|Default|SetSkyMaterial _returnvalue)
  (bind _returnvalue_2 (Class|SunLightSimulatorComponent|CreateLookUpTexture (Variables|Default|GetSunLightSimulator) 4096 50))
  (Rendering|Material|SetTextureParameterValue (Variables|Default|GetSkyMaterial) "LookUpMap" _returnvalue_2))

(fn UpdateSunDirection
  (Rendering|Material|SetVectorParameterValue (Variables|Default|GetSkyMaterial) "SunDirection" (Math|Conversions|ToLinearColor(Vector) (Math|Rotator|GetRotationXVector (Transformation|GetActorRotation (Variables|Default|GetSunLight)))) :!class /Script/Engine.MaterialInstanceDynamic))