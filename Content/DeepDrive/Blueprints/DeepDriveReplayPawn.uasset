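; DeepDriveReplayPawn is a free-flying pawn, named for replay use, with mouse navigation similar to the Unreal editor viewport.
; Button events maintain a MouseButtons bitmask that Update reads each Tick: left drag yaws and moves horizontally forward/back, right drag looks around, both pan sideways and vertically.
; Movement axes work only while a button is held, and the wheel steps along the view, both through Translate, which offsets location without sweeping.
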(event EventBeginPlay)

(event Collision|EventActorBeginOverlap
  (params (OtherActor :type Actor%20Object%20Reference)))

(event EventTick
  (params (DeltaSeconds :type Float%20%28single-precision%29))
  (bind _returnvalue (Game|GetPlayerController 0))
  (bind (_deltax _deltay) (Class|PlayerController|GetInputMouseDelta _returnvalue))
  (CallFunction|Update _deltax _deltay))

(event Input|AxisEvents|InputAxisMoveForward
  (params (AxisValue :type Float%20%28single-precision%29))
  (if (and (> (Math|Float|Absolute(Float) AxisValue) 0.01) (!= (Variables|Default|GetMouseButtons) 0))
    (CallFunction|Translate (Math|Vector|GetForwardVector (Pawn|GetControlRotation :!class /Script/Engine.Pawn)) (* AxisValue (Variables|Default|GetKeyboardMoveSens)))))

(event Input|AxisEvents|InputAxisMoveRight
  (params (AxisValue :type Float%20%28single-precision%29))
  (if (and (> (Math|Float|Absolute(Float) AxisValue) 0.01) (!= (Variables|Default|GetMouseButtons) 0))
    (CallFunction|Translate (Math|Vector|GetRightVector (Pawn|GetControlRotation :!class /Script/Engine.Pawn)) (* AxisValue (Variables|Default|GetKeyboardMoveSens)))))

(event Input|MouseEvents|LeftMouseButton
  (params (Key :type Key%20Structure))
  (:Pressed
    (Variables|Default|SetMouseButtons (Class|KismetMathLibrary|OrIntInt (Variables|Default|GetMouseButtons) 1)))
  (:Released
    (Variables|Default|SetMouseButtons (Class|KismetMathLibrary|AndIntInt (Variables|Default|GetMouseButtons) 2))))

(event Input|MouseEvents|RightMouseButton
  (params (Key :type Key%20Structure))
  (:Pressed
    (Variables|Default|SetMouseButtons (Class|KismetMathLibrary|OrIntInt (Variables|Default|GetMouseButtons) 2)))
  (:Released
    (Variables|Default|SetMouseButtons (Class|KismetMathLibrary|AndIntInt (Variables|Default|GetMouseButtons) 1))))

(event Input|MouseEvents|MouseWheelUp
  (params (Key :type Key%20Structure))
  (:Pressed
    (CallFunction|Translate (Math|Vector|GetForwardVector (Pawn|GetControlRotation :!class /Script/Engine.Pawn)) (Variables|Default|GetKeyboardMoveSens))))

(event Input|MouseEvents|MouseWheelDown
  (params (Key :type Key%20Structure))
  (:Pressed
    (CallFunction|Translate (Math|Vector|GetForwardVector (Pawn|GetControlRotation :!class /Script/Engine.Pawn)) (* -1.0 (Variables|Default|GetKeyboardMoveSens)))))

(fn ConstructionScript)

(fn Update
  (params (MouseDeltaX :type Float%20%28single-precision%29) (MouseDeltaY :type Float%20%28single-precision%29))
  (bind _returnvalue (Pawn|GetControlRotation :!class /Script/Engine.Pawn))
  (bind _returnvalue_2 (Math|Rotator|MakeRotator 0.0 0.0 (.yaw _returnvalue)))
  (switch int (Variables|Default|GetMouseButtons)
    (:1
      (Pawn|Input|AddControllerYawInput (* (Variables|Default|GetMouseRotateSens) MouseDeltaX))
      (Transformation|SetActorLocation (+ (Transformation|GetActorLocation) (* (Math|Vector|GetForwardVector (Math|Rotator|MakeRotator 0.0 0.0 (.Yaw (Math|Rotator|BreakRotator (Pawn|GetControlRotation :!class /Script/Engine.Pawn))))) (* MouseDeltaY (Variables|Default|GetMouseMoveSens)))) false false))
    (:2
      (Pawn|Input|AddControllerYawInput (* MouseDeltaX (Variables|Default|GetMouseRotateSens)))
      (Pawn|Input|AddControllerPitchInput (* MouseDeltaY (Variables|Default|GetMouseRotateSens) -1.0)))
    (:3
      (Transformation|SetActorLocation (+ (* (Math|Vector|GetRightVector _returnvalue_2) (* MouseDeltaX (Variables|Default|GetMouseMoveSens))) (* (Math|Vector|GetUpVector _returnvalue_2) (* MouseDeltaY (Variables|Default|GetMouseMoveSens))) (Transformation|GetActorLocation)) false false))))

(fn Translate
  (params (Direction :type Vector) (Value :type Float%20%28single-precision%29))
  (Transformation|SetActorLocation (+ (Transformation|GetActorLocation) (* Direction Value)) false false))