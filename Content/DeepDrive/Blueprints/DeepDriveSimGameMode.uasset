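; Game mode for the DeepDrive simulation that handles the loading screen and pause menu.
; BeginPlay optionally shows a loading screen, which OnSimulationReady fades out while fading in the simulation HUD.
; OnPause acts as a toggle keyed on the pause menu widget's existence, creating or removing it while switching game pause, input mode, mouse cursor and HUD instrument visibility.
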(event EventBeginPlay
  (if (Variables|Default|GetShowLoadingScreen)
    (bind _returnvalue (UserInterface|CreateWidget "/Game/DeepDrive/Simulation/HUD/LoadingScreenWidget.LoadingScreenWidget_C"))
    (bind _output_get (Variables|Default|SetLoadingScreen _returnvalue))
    (UserInterface|Viewport|AddtoViewport _output_get 0)))

(fn ConstructionScript)

(fn OnSimulationReady
  (Utilities|FlowControl|Sequence
    (:then_0
      (if (!= (Variables|Default|GetLoadingScreen) 0)
        (Default|FadeOut (Variables|Default|GetLoadingScreen) 2.0)))
    (:then_1
      (bind _asdeep_drive_simulation_hud (Utilities|Casting|CastToDeepDriveSimulationHUD (HUD|GetHUD (Game|GetPlayerController 0))))
      (Default|FadeinHUD _asdeep_drive_simulation_hud 2.0))))

(fn OnPause
  (bind _returnvalue (Game|GetPlayerController 0))
  (bind _returnvalue_2 (Game|GetPlayerController 0))
  (if (== (Variables|Default|GetPauseMenu) 0)
    (Utilities|FlowControl|Sequence
      (:then_0
        (bind _returnvalue_3 (UserInterface|CreateWidget "/Game/DeepDrive/Simulation/UI/PauseMenu/PauseMenu.PauseMenu_C"))
        (bind _output_get (Variables|Default|SetPauseMenu _returnvalue_3))
        (UserInterface|Viewport|AddtoViewport _output_get 0))
      (:then_1
        (Game|SetGamePaused true)
        (Input|SetInputModeGameandUI _returnvalue_2 0 "DoNotLock" true)
        (Variables|/Script/Engine.PlayerController|SetbShowMouseCursor _returnvalue_2 true))
      (:then_2
        (bind _asdeep_drive_simulation_hud (Utilities|Casting|CastToDeepDriveSimulationHUD (HUD|GetHUD (Game|GetPlayerController 0))))
        (Default|SetInstrumentsVisibility (Variables|/Game/DeepDrive/Simulation/HUD/DeepDriveSimulationHUD.DeepDriveSimulationHUD_C|GetHUDWidget _asdeep_drive_simulation_hud) false)))
    (else
      (Utilities|FlowControl|Sequence
        (:then_0
          (Widget|RemovefromParent (Variables|Default|GetPauseMenu))
          (Variables|Default|SetPauseMenu 0)
          (Game|SetGamePaused false))
        (:then_1
          (Input|SetInputModeGameOnly _returnvalue)
          (Variables|/Script/Engine.PlayerController|SetbShowMouseCursor _returnvalue false))
        (:then_2
          (bind _asdeep_drive_simulation_hud_2 (Utilities|Casting|CastToDeepDriveSimulationHUD (HUD|GetHUD (Game|GetPlayerController 0))))
          (Default|SetInstrumentsVisibility (Variables|/Game/DeepDrive/Simulation/HUD/DeepDriveSimulationHUD.DeepDriveSimulationHUD_C|GetHUDWidget _asdeep_drive_simulation_hud_2) true))))))