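; Input controller for the DeepDrive driving simulation that turns player input into simulator commands.
; Forwards movement, look, camera, mode, agent and debug inputs to DeepDriveSim; Flip resets the simulation while toggling additional agents.
; Sun controls go to DeepDriveSimLightingMgr, with time-of-day presets indexed by parsing the pressed key's display name as a number.
; The pause input calls OnPause on the game mode.
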(event Input|ActionEvents|InputActionChaseCam
  (params (Key :type Key%20Structure))
  ;[1 1 1] Forward Camera Selection to DeepDriveSim
  (:Pressed
    (Class|DeepDriveSimulation|SelectCamera (Variables|Default|GetDeepDriveSim) "CHASE_CAMERA")))

(event Input|ActionEvents|InputActionRemoteAI
  (params (Key :type Key%20Structure))
  ;[1 1 1] Switch Modes
  (:Pressed
    (Class|DeepDriveSimulation|SelectMode (Variables|Default|GetDeepDriveSim) "REMOTE_AI")))

(event Input|ActionEvents|InputActionNextAgent
  (params (Key :type Key%20Structure))
  ;[1 1 1] Agents
  (:Pressed
    (Class|DeepDriveSimulation|NextAgent (Variables|Default|GetDeepDriveSim))))

(event Input|ActionEvents|InputActionPrevAgent
  (params (Key :type Key%20Structure))
  ;[1 1 1] Agents
  (:Pressed
    (Class|DeepDriveSimulation|PreviousAgent (Variables|Default|GetDeepDriveSim))))

(event Input|ActionEvents|InputActionFlip
  (params (Key :type Key%20Structure))
  ;[1 1 1] Agents
  (:Pressed
    (Class|DeepDriveSimulation|ResetSimulation (Variables|Default|GetDeepDriveSim) (Variables|Default|GetHasAdditionalAgents))
    (Variables|Default|SetHasAdditionalAgents (not (Variables|Default|GetHasAdditionalAgents)))))

(event Input|ActionEvents|InputActionPauseMenu
  (params (Key :type Key%20Structure))
  (:Pressed
    (bind _asdeep_drive_sim_game_mode (Utilities|Casting|CastToDeepDriveSimGameMode (Game|GetGameMode)))
    (Default|OnPause _asdeep_drive_sim_game_mode)))

(event Input|ActionEvents|InputActionDayTime
  (params (Key :type Key%20Structure))
  (bind _returnvalue (Class|KismetInputLibrary|KeyGetDisplayName Key))
  (bind _daytimes (Variables|Default|GetDayTimes))
  (bind _returnvalue_2 (Utilities|String|ToString(Text) _returnvalue))
  (bind _returnvalue_3 (Math|Conversions|ToInteger(Byte) _returnvalue_2))
  (bind _returnvalue_4 (- _returnvalue_3 1))
  (bind _output (Utilities|Array|Get(acopy) _daytimes _returnvalue_4))
  ;[1 1 1] Time of Day
  (:Pressed
    (Default|SetTime (Variables|Default|GetDeepDriveSimLightingMgr) (.x _output) (.y _output) 2.0)))

(event Input|ActionEvents|InputActionToggleAgentRenderMode
  (params (Key :type Key%20Structure))
  (:Pressed
    (Class|DeepDriveSimulation|ToggleAgentRenderMode (Variables|Default|GetDeepDriveSim))))

(event Input|ActionEvents|InputActionInteriorCam
  (params (Key :type Key%20Structure))
  ;[1 1 1] Forward Camera Selection to DeepDriveSim
  (:Pressed
    (Class|DeepDriveSimulation|SelectCamera (Variables|Default|GetDeepDriveSim) "INTERIOR_CAMERA")))

(event Input|ActionEvents|InputActionToggleCollisionMode
  (params (Key :type Key%20Structure))
  (:Pressed
    (Class|DeepDriveSimulation|ToggleAgentCollisionMode (Variables|Default|GetDeepDriveSim))))

(event Input|ActionEvents|InputActionManualMode
  (params (Key :type Key%20Structure))
  ;[1 1 1] Switch Modes
  (:Pressed
    (Class|DeepDriveSimulation|SelectMode (Variables|Default|GetDeepDriveSim) "MANUAL")))

(event Input|ActionEvents|InputActionSplineMode
  (params (Key :type Key%20Structure))
  ;[1 1 1] Switch Modes
  (:Pressed
    (Class|DeepDriveSimulation|SelectMode (Variables|Default|GetDeepDriveSim) "LOCAL_AI")))

(event Input|ActionEvents|InputActionToggleSunSimulation
  (params (Key :type Key%20Structure))
  ;[1 1 1] Sun Simulation
  (:Pressed
    (Default|ToggleSunSimulation (Variables|Default|GetDeepDriveSimLightingMgr))))

(event Input|ActionEvents|InputActionToggleCollisionVisibility
  (params (Key :type Key%20Structure))
  (:Pressed
    (Class|DeepDriveSimulation|ToggleCollisionVisibility (Variables|Default|GetDeepDriveSim))))

(event Input|ActionEvents|InputActionIncreaseSunSimulationSpeed
  (params (Key :type Key%20Structure))
  ;[1 1 1] Sun Simulation
  (:Pressed
    (Default|IncreaseSimulationSpeed (Variables|Default|GetDeepDriveSimLightingMgr))))

(event Input|ActionEvents|InputActionDecreaseSunSimutlationSpeed
  (params (Key :type Key%20Structure))
  ;[1 1 1] Sun Simulation
  (:Pressed
    (Default|DecreaseSimulationSpeed (Variables|Default|GetDeepDriveSimLightingMgr))))

(event Input|ActionEvents|InputActionDebugTrigger
  (params (Key :type Key%20Structure))
  ;[1 1 1] Debug
  (:Pressed
    (Class|DeepDriveSimulation|OnDebugTrigger (Variables|Default|GetDeepDriveSim))))

(event Input|ActionEvents|InputActionOrbitCam
  (params (Key :type Key%20Structure))
  ;[1 1 1] Forward Camera Selection to DeepDriveSim
  (:Pressed
    (Class|DeepDriveSimulation|SelectCamera (Variables|Default|GetDeepDriveSim) "ORBIT_CAMERA")))

(event Input|ActionEvents|InputActionFreeCamera
  (params (Key :type Key%20Structure))
  ;[1 1 1] Forward Camera Selection to DeepDriveSim
  (:Pressed
    (Class|DeepDriveSimulation|SelectCamera (Variables|Default|GetDeepDriveSim) "FREE_CAMERA")))

(event Input|AxisEvents|InputAxisMoveForward
  (params (AxisValue :type Float%20%28single-precision%29))
  ;[1 1 1] Forward Control Input to DeepDriveSim
  (Class|DeepDriveSimulation|MoveForward (Variables|Default|GetDeepDriveSim) AxisValue))

(event Input|AxisEvents|InputAxisLookUp
  (params (AxisValue :type Float%20%28single-precision%29))
  ;[1 1 1] Forward Control Input to DeepDriveSim
  (Class|DeepDriveSimulation|LookUp (Variables|Default|GetDeepDriveSim) AxisValue))

(event Input|AxisEvents|InputAxisLookUp
  (params (AxisValue :type Float%20%28single-precision%29))
  ;[1 1 1] Forward Control Input to DeepDriveSim
  (Class|DeepDriveSimulation|LookUp (Variables|Default|GetDeepDriveSim) AxisValue))

(event Input|AxisEvents|InputAxisTurn
  (params (AxisValue :type Float%20%28single-precision%29))
  ;[1 1 1] Forward Control Input to DeepDriveSim
  (Class|DeepDriveSimulation|Turn (Variables|Default|GetDeepDriveSim) AxisValue))

(event Input|AxisEvents|InputAxisTurn
  (params (AxisValue :type Float%20%28single-precision%29))
  ;[1 1 1] Forward Control Input to DeepDriveSim
  (Class|DeepDriveSimulation|Turn (Variables|Default|GetDeepDriveSim) AxisValue))

(event Input|AxisEvents|InputAxisMoveRight
  (params (AxisValue :type Float%20%28single-precision%29))
  ;[1 1 1] Forward Control Input to DeepDriveSim
  (Class|DeepDriveSimulation|MoveRight (Variables|Default|GetDeepDriveSim) AxisValue))

(fn ConstructionScript)