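; DeepDriveUtils is a utility Blueprint providing a SmoothStep function for easing a value between two edges.
; It normalises X between Edge0 and Edge1 and clamps the result to the 0–1 range as T.
; A math expression node holds the cubic Hermite polynomial T²(3 − 2T) that gives the smooth S-curve.
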(fn SmoothStep
  (params (Edge0 :type Float%20%28single-precision%29) (Edge1 :type Float%20%28single-precision%29) (X :type Float%20%28single-precision%29))
  (Utilities|FlowControl|Sequence
    (:then_0
      (LocalVariables|SetT (Math|Float|Clamp(Float) (/ (- X Edge0) (- Edge1 Edge0)))))
    (:then_1
      (return (|(({C817F938-47CF-5BDE-F875-3A800148E7C2}*{C817F938-47CF-5BDE-F875-3A800148E7C2})*(3.000000-(2.000000*{C817F938-47CF-5BDE-F875-3A800148E7C2}))))))))